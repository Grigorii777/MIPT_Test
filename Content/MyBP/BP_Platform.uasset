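; BP_Platform is a platform actor that shuttles back and forth along a direction vector in discrete steps.
; From BeginPlay, a looping Delay chain offsets it by Dir without sweep, prints a debug "Hello", waits 1/Speed seconds, then updates StepCount.
; When the count exceeds Ampl or drops below zero, it negates Dir and flips DirStep to reverse both movement and counting.
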(event EventBeginPlay
  (bind _stepcount (Variables|Default|GetStepCount))
  (CallFunction|Move (Variables|Default|GetDir) :!label _label)
  (Development|PrintString "Hello")
  (Utilities|FlowControl|Delay (/ 1.0 (Variables|Default|GetSpeed)))
  (CallFunction|AddStep)
  (if (> _stepcount (Variables|Default|GetAmpl))
    _
    (elif (< _stepcount 0)
      _
      (else
        (goto _label))))
  (Variables|Default|SetDirStep (not (Variables|Default|GetDirStep)))
  (Variables|Default|SetDir (* (Variables|Default|GetDir) -1.0))
  (goto _label))

(event Collision|EventActorBeginOverlap
  (params (OtherActor :type Actor%20Object%20Reference)))

(fn ConstructionScript)

(fn Move
  (params (Dir :type Vector))
  (Transformation|AddActorWorldOffset self Dir))

(fn AddStep
  (if (Variables|Default|GetDirStep)
    (bind _result (Math|Integer|IncrementInt (Variables|Default|GetStepCount))
      (:%20%20
        (Variables|Default|SetStepCount _result)))
    (else
      (Math|Integer|DecrementInt (Variables|Default|GetStepCount)
        (:%20%20
          (Variables|Default|SetStepCount (Variables|Default|GetStepCount)))))))